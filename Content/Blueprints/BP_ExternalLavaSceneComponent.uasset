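; External lava scene component that makes a lava decal gradually start flowing on demand.
; On BeginPlay it creates a dynamic material on its first child decal, applying opacity and flow speed with the opacity offset at full.
; StartFlowing waits a random delay, then eases that offset linearly to zero through a next-tick delay loop, over a duration derived from flow speed.
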(event Custom|StartFlowing
  (Utilities|FlowControl|Delay (Math|Random|RandomFloatinRange 0.0 1e+01))
  (Variables|Default|SettimeToSetFullFlow (* (+ 1.0 (* (Variables|Default|GetflowSpeed) -1e+01)) 5.0))
  (Variables|Default|SetflowStartTime (Utilities|Time|GetGameTimeinSeconds))
  (bind _output_get (Variables|Default|SetopacityOffset (Math|Float|MapRangeClamped (- (Utilities|Time|GetGameTimeinSeconds) (Variables|Default|GetflowStartTime)) 0.0 (Variables|Default|GettimeToSetFullFlow) 1.0 0.0) :!label _label))
  (Rendering|Material|SetScalarParameterValue (Variables|Default|GetdecalMaterialInstance) "opacityOffset" _output_get :!class /Script/Engine.MaterialInstanceDynamic)
  (if (== (Variables|Default|GetopacityOffset) 0.0)
    (Development|PrintString "start flowing completed")
    (else
      (Utilities|FlowControl|DelayUntilNextTick)
      (goto _label))))

(event Custom|CustomEvent)

(event EventBeginPlay
  (bind _asdecal_component (Utilities|Casting|CastToDecalComponent (Components|GetChildComponent 0)))
  (bind _returnvalue (Rendering|Material|CreateDynamicMaterialInstance _asdecal_component :!class /Script/Engine.DecalComponent))
  (bind _output_get (Variables|Default|SetdecalMaterialInstance _returnvalue))
  (Rendering|Material|SetScalarParameterValue _output_get "Opacity" (Variables|Default|Getopacity) :!class /Script/Engine.MaterialInstanceDynamic)
  (Rendering|Material|SetScalarParameterValue _returnvalue "flowSpeedY" (Variables|Default|GetflowSpeed) :!class /Script/Engine.MaterialInstanceDynamic)
  (Rendering|Material|SetScalarParameterValue _returnvalue "opacityOffset" 1.0 :!class /Script/Engine.MaterialInstanceDynamic))

(event EventTick
  (params (DeltaSeconds :type Float%20%28single-precision%29)))