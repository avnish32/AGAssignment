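; Camera controller that drives a cine camera's location, rotation and FOV every Tick, clamping height between min and max Z.
; Four preset events jump to stored viewpoints around the volcano, house, forest and lake.
; BeginPlay and presets mirror location and rotation to a UI by HTTP PUT of JSON property writes on this actor's own path, apparently through Remote Control.
; Focus and aperture setters exist but never run.
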(event Custom|Cam%204%20-%20Facing%20the%20lake%20on%20the%20forest%20edge
  (bind _cam4transform (Variables|CameraPresets|Getcam4Transform))
  (bind _returnvalue (CallFunction|MakeCameraTransform (.location _cam4transform) (.rotation _cam4transform)))
  (Variables|Default|SetcameraLocation (.location _returnvalue))
  (Variables|Default|SetcameraRotation (.rotation _returnvalue))
  (CallFunction|ReplicateCamLocationonUI)
  (CallFunction|ReplicateCamRotationonUI))

(event Custom|Cam%201%20-%20Looking%20at%20the%20volcano%20from%20the%20house
  (bind _cam1transform (Variables|cameraPresets|Getcam1Transform))
  (bind _returnvalue (CallFunction|MakeCameraTransform (.location _cam1transform) (.rotation _cam1transform)))
  (Variables|Default|SetcameraLocation (.location _returnvalue))
  (Variables|Default|SetcameraRotation (.rotation _returnvalue))
  (CallFunction|ReplicateCamLocationonUI)
  (CallFunction|ReplicateCamRotationonUI))

(event Custom|ReplicateCamLocationOnUI
  (bind _outjsonstring (CallFunction|GetJSONReqforCamLocation (Variables|Default|GetcameraLocation)))
  (bind _result_body (|HttpRequest (Variables|Default|GetRCHttpPutPropertyURL) "Put" (|MakeRequestHeader "Json") _outjsonstring)
    (:On%20Success
      (Development|PrintString (Utilities|String|Append _result_body "Cam location Req success")))
    (:On%20Error
      (Development|PrintString "Cam location Req failed"))))

(event Custom|ReplicateCamRotationOnUI
  (bind _outjsonstring (CallFunction|GetJSONReqforCamRotation (Variables|Default|GetcameraRotation)))
  (bind _result_body (|HttpRequest (Variables|Default|GetRCHttpPutPropertyURL) "Put" (|MakeRequestHeader "Json") _outjsonstring)
    (:On%20Success
      (Development|PrintString (Utilities|String|Append _result_body "Cam rotation Req success")))
    (:On%20Error
      (Development|PrintString "Cam rotation Req failed"))))

(event Custom|Cam%202%20-%20Looking%20at%20the%20volcano%20from%20the%20flower%20field
  (bind _cam2transform (Variables|CameraPresets|Getcam2Transform))
  (bind _returnvalue (CallFunction|MakeCameraTransform (.location _cam2transform) (.rotation _cam2transform)))
  (Variables|Default|SetcameraLocation (.location _returnvalue))
  (Variables|Default|SetcameraRotation (.rotation _returnvalue))
  (CallFunction|ReplicateCamLocationonUI)
  (CallFunction|ReplicateCamRotationonUI))

(event Custom|Cam%203%20-%20Facing%20the%20volcano%20inside%20the%20forest
  (bind _cam3transform (Variables|CameraPresets|Getcam3Transform))
  (bind _returnvalue (CallFunction|MakeCameraTransform (.location _cam3transform) (.rotation _cam3transform)))
  (Variables|Default|SetcameraLocation (.location _returnvalue))
  (Variables|Default|SetcameraRotation (.rotation _returnvalue))
  (CallFunction|ReplicateCamLocationonUI)
  (CallFunction|ReplicateCamRotationonUI))

(event EventBeginPlay
  (bind _camera (Variables|Default|Getcamera))
  (bind _returnvalue (Transformation|GetActorTransform _camera))
  (Variables|Default|SetcameraLocation (.location _returnvalue))
  (Variables|Default|SetcameraRotation (.rotation _returnvalue))
  (CallFunction|ReplicateCamLocationonUI)
  (CallFunction|ReplicateCamRotationonUI))

(event EventTick
  (params (DeltaSeconds :type Float%20%28single-precision%29))
  (bind _camera (Variables|Default|Getcamera))
  (bind _returnvalue (CallFunction|MakeCameraTransform (Variables|Default|GetcameraLocation) (Variables|Default|GetcameraRotation)))
  (Transformation|SetActorTransform _camera _returnvalue)
  (Camera|SetFieldOfView (Variables|/Game/FirstPerson/Blueprints/BP_FirstPersonCharacter.BP_FirstPersonCharacter_C|GetCineCamera _camera) (Variables|Default|GetFOV)))

(fn ConstructionScript)

(fn MakeCameraTransform
  (params (location :type Vector) (rotation :type Rotator))
  (return (Math|Transform|MakeTransform (Math|Vector|MakeVector (.x location) (.y location) (Math|Float|Clamp(Float) (.z location) (Variables|Default|GetminZPosition) (Variables|Default|GetmaxZPosition))) rotation)))

(fn GetJSONReqforCamLocation
  (params (camLocation :type Vector))
  (bind _outjsonstring (|StructtoJsonString (Utilities|Struct|MakeS_CamLocationWriteCall (Class|KismetSystemLibrary|GetPathName self) "WRITE_ACCESS" "cameraLocation" (Utilities|Struct|MakeS_CamLocation camLocation))))
  (return _outjsonstring))

(fn GetJSONReqforCamRotation
  (params (camRotation :type Rotator))
  (bind _outjsonstring (|StructtoJsonString (Utilities|Struct|MakeS_CamRotationWriteCall (Class|KismetSystemLibrary|GetPathName self) "WRITE_ACCESS" "cameraRotation" (Utilities|Struct|MakeS_CamRotation camRotation))))
  (return _outjsonstring))