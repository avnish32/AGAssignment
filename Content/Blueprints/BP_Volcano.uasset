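; Volcano actor with a smoke plume that can erupt and be reset.
; Erupt removes the smoke, plays two camera shakes, fires explosion effects and starts its external lava components flowing.
; A per-tick loop raises the internal lava while cross-fading two dynamic materials' opacity, then respawns the smoke.
; ResetVolcano restores lava height, opacities and flows; the weather-based wind adjustment for smoke is never executed.
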(event Custom|Erupt
  (Components|DestroyComponent (Variables|Default|GetSmokeSystem))
  (Camera|PlayWorldCameraShake "/Game/FX/CamShake_VolcanoEruption.CamShake_VolcanoEruption_C" (Transformation|GetActorLocation) 0.0 1e+06)
  (Utilities|FlowControl|Delay 1.0)
  (Camera|PlayWorldCameraShake "/Game/FX/CamShake_VolcanoEruption.CamShake_VolcanoEruption_C" (Transformation|GetActorLocation) 0.0 1e+06)
  (Components|Activation|Activate (Variables|Default|GetExplosion_Vertical) true)
  (Components|Activation|Activate (Variables|Default|GetExplosion_Divergent) true)
  (for _array_element (Actor|GetComponentsByClass "/Game/Blueprints/BP_ExternalLavaSceneComponent.BP_ExternalLavaSceneComponent_C")
    (Default|StartFlowing _array_element)
    (Development|PrintString "StartFlowing called"))
  (bind _returnvalue (CallFunction|ShouldInternalLavabeLifted 3.5e+02 :!label _label))
  (if _returnvalue
    (CallFunction|LiftInternalLavaPerTick (Variables|/Script/Engine.SceneComponent|GetRelativeLocation (Variables|Default|GetInternalLava)) 5.0 3.5e+02)
    (Utilities|FlowControl|DelayUntilNextTick)
    (goto _label)
    (else
      (Development|PrintString "volcano eruption completed")
      (CallFunction|SpawnSmokeSystem))))

(event Custom|ResetVolcano
  (bind _internallava (Variables|Default|GetInternalLava))
  (bind _relativelocation (Variables|/Script/Engine.SceneComponent|GetRelativeLocation _internallava))
  (Transformation|SetRelativeLocation _internallava (Math|Vector|MakeVector (.x _relativelocation) (.y _relativelocation) 3.1e+02) false false)
  (Rendering|Material|SetScalarParameterValue (Variables|Default|GetinternalLavaDynamicMaterialInstance) "Opacity" 1.0 :!class /Script/Engine.MaterialInstanceDynamic)
  (Variables|Default|SetinternalLavaCurrentOpacity 1.0)
  (Rendering|Material|SetScalarParameterValue (Variables|Default|GetinternalLavaRisenMaterialInstance) "Opacity" 0.0 :!class /Script/Engine.MaterialInstanceDynamic)
  (Variables|Default|SetinternalLavaRisenCurrentOpacity 0.0)
  (for _array_element (Actor|GetComponentsByClass "/Game/Blueprints/BP_ExternalLavaSceneComponent.BP_ExternalLavaSceneComponent_C")
    (Default|Reset _array_element))
  (Development|PrintString "Volcano resetting completed"))

(event EventBeginPlay
  (CallFunction|SpawnSmokeSystem)
  (bind _returnvalue (Rendering|Material|CreateDynamicMaterialInstance (Variables|Default|GetInternalLava) 0 "/Game/Materials/Volcano/M_InternalLava.M_InternalLava" "None" :!class /Script/Engine.PrimitiveComponent))
  (Variables|Default|SetinternalLavaDynamicMaterialInstance _returnvalue)
  (bind _returnvalue_2 (Rendering|Material|CreateDynamicMaterialInstance (Variables|Default|GetIntLavaRisen) :!class /Script/Engine.DecalComponent))
  (Variables|Default|SetinternalLavaRisenMaterialInstance _returnvalue_2)
  (bind _returnvalue_3 (Actor|GetActorOfClass "/Game/Blueprints/BP_Weather.BP_Weather_C"))
  (Variables|Default|SetweatherSystem _returnvalue_3))

(event EventTick
  (params (DeltaSeconds :type Float%20%28single-precision%29)))

(fn ConstructionScript)

(fn SpawnSmokeSystem
  (bind _returnvalue (Niagara|SpawnSystematLocation "/Game/FX/NS_Smoke2D.NS_Smoke2D" (+ (Transformation|GetActorLocation) "750.000000,-200.000000,3250.000000")))
  (Variables|Default|SetSmokeSystem _returnvalue))

(fn ShouldInternalLavabeLifted
  (params (endPosition :type Float%20%28double-precision%29))
  (return (not (== (.z (Variables|/Script/Engine.SceneComponent|GetRelativeLocation (Variables|Default|GetInternalLava))) endPosition))))

(fn LiftInternalLavaPerTick
  (params (currentLocationIn :type Vector) (timeToTakeToLift :type Float%20%28double-precision%29) (endPosition :type Float%20%28double-precision%29))
  (Transformation|SetRelativeLocation (Variables|Default|GetInternalLava) (Math|Vector|MakeVector (.x currentLocationIn) (.y currentLocationIn) (Math|Interpolation|FInterptoConstant (.z currentLocationIn) endPosition (Utilities|Time|GetWorldDeltaSeconds) (/ 4e+01 timeToTakeToLift))) false false)
  (Development|PrintString (Utilities|String|ToString(Float) (Math|Interpolation|FInterptoConstant (Variables|Default|GetinternalLavaCurrentOpacity) 0.0 (Utilities|Time|GetWorldDeltaSeconds) (/ 1.0 timeToTakeToLift))))
  (bind _output_get (Variables|Default|SetinternalLavaCurrentOpacity (Math|Interpolation|FInterptoConstant (Variables|Default|GetinternalLavaCurrentOpacity) 0.0 (Utilities|Time|GetWorldDeltaSeconds) (/ 1.0 timeToTakeToLift))))
  (Rendering|Material|SetScalarParameterValue (Variables|Default|GetinternalLavaDynamicMaterialInstance) "Opacity" _output_get :!class /Script/Engine.MaterialInstanceDynamic)
  (Rendering|Material|SetScalarParameterValue (Variables|Default|GetinternalLavaRisenMaterialInstance) "Opacity" (Math|Interpolation|FInterptoConstant (Variables|Default|GetinternalLavaRisenCurrentOpacity) 1.0 (Utilities|Time|GetWorldDeltaSeconds) (/ 1.0 timeToTakeToLift)) :!class /Script/Engine.MaterialInstanceDynamic)
  (Variables|Default|SetinternalLavaRisenCurrentOpacity (Math|Interpolation|FInterptoConstant (Variables|Default|GetinternalLavaRisenCurrentOpacity) 1.0 (Utilities|Time|GetWorldDeltaSeconds) (/ 1.0 timeToTakeToLift)))
  (return))