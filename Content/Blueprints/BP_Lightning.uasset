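; Lightning actor that strikes at random positions in the sky around the player, with delayed thunder.
; Each strike turns toward the player, picks one of two bolt textures, then a timeline animates material mask offsets and emission.
; The timeline also flashes post-process exposure, restoring the saved settings afterwards.
; A randomly delayed BeginPlay loop triggers strikes while the owning BP_Weather enables auto lightning; StrikeWithSound blocks overlapping calls.
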(event Custom|Strike
  (bind _lightningplane (Variables|Default|GetLightningPlane))
  (bind _ppvolume (Variables|Default|GetPPVolume))
  (CallFunction|SetRandomLocation)
  (CallFunction|SetLightningTexture)
  (Variables|Default|SetoriginalPostProcessSettings (Variables|/Script/Engine.PostProcessVolume|GetSettings (Variables|Default|GetPPVolume)))
  (bind (_direction _xoffset _yoffset _emission _exposure) (Timeline|TL_Lightning PlayFromStart)
    (:Update
      (Rendering|Material|SetScalarParameterValueonMaterials _lightningplane "opacityMaskOffsetX" _xoffset)
      (Rendering|Material|SetScalarParameterValueonMaterials _lightningplane "opacityMaskOffsetY" _yoffset)
      (Rendering|Material|SetScalarParameterValueonMaterials _lightningplane "emission" _emission)
      (Utilities|IsValid _ppvolume
        (:Is%20Valid
          (Variables|/Script/Engine.PostProcessVolume|SetSettings _ppvolume (Utilities|Struct|MakePostProcessSettings "AEM_Manual" (* _exposure (Math|Float|Absolute(Float) (Utilities|Struct|BreakPostProcessSettings (Variables|Default|GetoriginalPostProcessSettings)))))))
        (:Is%20Not%20Valid
          (Development|PrintString "PPVolume not set on BP_Lightning"))))
    (:Finished
      (Variables|/Script/Engine.PostProcessVolume|SetSettings (Variables|Default|GetPPVolume) (Variables|Default|GetoriginalPostProcessSettings)))))

(event Custom|StrikeWithSound
  (if (Variables|Default|GetcanStrike)
    (Variables|Default|SetcanStrike false)
    (CallFunction|Strike)
    (Utilities|FlowControl|Delay 1.0)
    (Audio|PlaySound2D "/Game/FX/mixkit-cinematic-thunder-1283.mixkit-cinematic-thunder-1283" 1.0 1.0 0.0 0 0)
    (Variables|Default|SetcanStrike true)))

(event EventBeginPlay
  (Utilities|IsValid (Variables|Default|GetPPVolume)
    (:Is%20Not%20Valid
      (bind _returnvalue (Actor|GetActorOfClass "/Script/Engine.PostProcessVolume"))
      (Variables|Default|SetPPVolume _returnvalue)
      (Utilities|FlowControl|Delay (Math|Random|RandomFloatinRange 4.0 1e+01) :!label _label)
      (bind _asbp_weather (Utilities|Casting|CastToBP_Weather (Components|GetOwner)))
      (if (Variables|/Game/Blueprints/BP_Weather.BP_Weather_C|GettoggleAutoLightningStrikes _asbp_weather)
        (Development|PrintString "auto lightning true in bp_lightning")
        (CallFunction|StrikewithSound)
        (goto _label)))))

(event EventTick
  (params (DeltaSeconds :type Float%20%28single-precision%29)))

(fn ConstructionScript)

(fn SetRandomLocation
  (bind _returnvalue (Game|GetPlayerCharacter 0))
  (bind _returnvalue_2 (Transformation|GetActorLocation _returnvalue))
  (Transformation|SetActorLocation (+ _returnvalue_2 (Math|Vector|MakeVector (Math|Random|RandomFloatinRange -4e+04 4e+04) (Math|Random|RandomFloatinRange -4e+04 4e+04) (Math|Random|RandomFloatinRange 1e+04 1.5e+04))) false false)
  (Transformation|SetActorRotation (Math|Rotator|MakeRotator 0.0 0.0 (.yaw (Math|Rotator|FindLookatRotation (Transformation|GetActorLocation) _returnvalue_2))))
  (return))

(fn SetLightningTexture
  (Utilities|IsValid (Variables|Default|GetlightingMaterialInstance)
    (:Is%20Valid
      _)
    (:Is%20Not%20Valid
      (bind _returnvalue (Rendering|Material|CreateDynamicMaterialInstance (Variables|Default|GetLightningPlane) 0 "/Game/Materials/Lightning/M_Lightning.M_Lightning" "None" :!class /Script/Engine.PrimitiveComponent))
      (Variables|Default|SetlightingMaterialInstance _returnvalue)))
  (Rendering|Material|SetTextureParameterValue (Variables|Default|GetlightingMaterialInstance) "lightningTexture" (Utilities|Select :Index (Math|Random|RandomIntegerinRange 0 1) :Option%200 "/Game/Materials/Lightning/pngimg_com_-_lightning_PNG5.pngimg_com_-_lightning_PNG5" :Option%201 "/Game/Materials/Lightning/pngimg_com_-_lightning_PNG25.pngimg_com_-_lightning_PNG25"))
  (return))