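; Weather controller actor that blends the level's atmosphere between presets such as dark and normal, with a rain toggle.
; BeginPlay finds the cloud, post-process and sky actors and maps presets to parameters.
; Preset changes enable Tick, which interpolates cloud density, exposure and Rayleigh scattering at constant speed, then disables itself once exposure reaches target.
; Rain toggling also sets wetness in a global material parameter collection.
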(event Custom|Dark
  (CallFunction|CheckandChangeAtmosphere "NewEnumerator0"))

(event Custom|Normal
  (CallFunction|CheckandChangeAtmosphere "NewEnumerator1"))

(event Custom|ToggleRain
  (if (Variables|Default|GetisRaining)
    (Rendering|Material|SetScalarParameterValue "/Game/Materials/MPC_Global.MPC_Global" "Wetness" 0.0 :!class /Script/Engine.KismetMaterialLibrary)
    (CallFunction|Normal)
    (else
      (Rendering|Material|SetScalarParameterValue "/Game/Materials/MPC_Global.MPC_Global" "Wetness" (Variables|Default|GetrainWetness) :!class /Script/Engine.KismetMaterialLibrary)
      (CallFunction|Dark)))
  (Variables|Default|SetisRaining (not (Variables|Default|GetisRaining))))

(event EventBeginPlay
  (Utilities|FlowControl|Sequence
    (:then_0
      (bind _returnvalue (Actor|GetActorOfClass "/Script/Engine.VolumetricCloud"))
      (Variables|WeatherControllers|SetVolumetricCloud _returnvalue))
    (:then_1
      (bind _returnvalue_2 (Actor|GetActorOfClass "/Script/Engine.PostProcessVolume"))
      (Variables|weatherControllers|SetPostProcessVolume _returnvalue_2))
    (:then_2
      (bind _returnvalue_3 (Actor|GetActorOfClass "/Script/Engine.SkyAtmosphere"))
      (Variables|WeatherControllers|SetSkyAtmosphere _returnvalue_3))
    (:then_3
      (bind _returnvalue_4 (Rendering|Material|CreateDynamicMaterialInstance "/Game/Materials/MI_SimpleVolumetricCloud.MI_SimpleVolumetricCloud" "None" "None" :!class /Script/Engine.KismetMaterialLibrary))
      (Variables|WeatherControllers|SetcloudMaterial _returnvalue_4))
    (:then_4
      (for _array_element (Variables|Default|GetweatherPresets)
        (Utilities|Map|Add (Variables|Default|GetweatherPresetToParamsMap) (.weatherPreset (Utilities|Struct|BreakWeatherParams _array_element)) _array_element)))
    (:then_5
      (Variables|Default|SetcurrentWeatherParams (.Value (Utilities|Map|Find (Variables|Default|GetweatherPresetToParamsMap) (Variables|Default|GetcurrentWeatherPreset)))))))

(event EventTick
  (params (DeltaSeconds :type Float%20%28single-precision%29))
  (CallFunction|ChangeAtmosphere (Variables|Default|GettargetWeatherPreset)))

(fn ConstructionScript)

(fn ChangeAtmosphere
  (params (weatherPreset :type WeatherPresets%20Enum :default "NewEnumerator0"))
  (bind _volumetriccloud (Variables|WeatherControllers|GetVolumetricCloud))
  (bind _skyatmosphere (Variables|WeatherControllers|GetSkyAtmosphere))
  (bind _postprocessvolume (Variables|weatherControllers|GetPostProcessVolume))
  (Utilities|FlowControl|Sequence
    (:then_0
      (LocalVariables|SettargetWeatherParams (.Value (Utilities|Map|Find (Variables|Default|GetweatherPresetToParamsMap) weatherPreset))))
    (:then_1
      (Utilities|IsValid _volumetriccloud
        (:Is%20Valid
          (Utilities|IsValid (Variables|WeatherControllers|GetcloudMaterial)
            (:Is%20Valid
              _)
            (:Is%20Not%20Valid
              (bind _returnvalue (Rendering|Material|CreateDynamicMaterialInstance "/Engine/EngineSky/VolumetricClouds/m_SimpleVolumetricCloud_Inst.m_SimpleVolumetricCloud_Inst" "None" "None" :!class /Script/Engine.KismetMaterialLibrary))
              (Variables|WeatherControllers|SetcloudMaterial _returnvalue)))
          (Rendering|Material|SetMaterial (Variables|/Script/Engine.VolumetricCloud|GetVolumetricCloudComponent _volumetriccloud) (Variables|WeatherControllers|GetcloudMaterial))
          (Rendering|Material|SetScalarParameterValue (Variables|WeatherControllers|GetcloudMaterial) "DensityModifier" (Math|Interpolation|FInterptoConstant (.cloudDensityModifier (Utilities|Struct|BreakWeatherParams (Variables|Default|GetcurrentWeatherParams))) (.cloudDensityModifier (Utilities|Struct|BreakWeatherParams (LocalVariables|GettargetWeatherParams))) (Utilities|Time|GetWorldDeltaSeconds) (Variables|Default|GetweatherChangeSpeed)) :!class /Script/Engine.MaterialInstanceDynamic)
          (Utilities|Struct|SetmembersinWeatherParams (Variables|Default|GetcurrentWeatherParams) (Math|Interpolation|FInterptoConstant (.cloudDensityModifier (Utilities|Struct|BreakWeatherParams (Variables|Default|GetcurrentWeatherParams))) (.cloudDensityModifier (Utilities|Struct|BreakWeatherParams (LocalVariables|GettargetWeatherParams))) (Utilities|Time|GetWorldDeltaSeconds) (Variables|Default|GetweatherChangeSpeed)) (CallFunction|ColorFinterptoConstant (.rayleighScattering (Utilities|Struct|BreakWeatherParams (Variables|Default|GetcurrentWeatherParams))) (.rayleighScattering (Utilities|Struct|BreakWeatherParams (LocalVariables|GettargetWeatherParams))) (Variables|Default|GetweatherChangeSpeed)) (Math|Interpolation|FInterptoConstant (.exposureCompensation (Utilities|Struct|BreakWeatherParams (Variables|Default|GetcurrentWeatherParams))) (.exposureCompensation (Utilities|Struct|BreakWeatherParams (LocalVariables|GettargetWeatherParams))) (Utilities|Time|GetWorldDeltaSeconds) (Variables|Default|GetweatherChangeSpeed)))
          (if (== (Math|Interpolation|FInterptoConstant (.exposureCompensation (Utilities|Struct|BreakWeatherParams (Variables|Default|GetcurrentWeatherParams))) (.exposureCompensation (Utilities|Struct|BreakWeatherParams (LocalVariables|GettargetWeatherParams))) (Utilities|Time|GetWorldDeltaSeconds) (Variables|Default|GetweatherChangeSpeed)) (.exposurecompensation (LocalVariables|GettargetWeatherParams)))
            (Development|PrintString "target expcomp")
            (Development|PrintString (Utilities|String|ToString(Float) (.exposurecompensation (LocalVariables|GettargetWeatherParams))))
            (Development|PrintString "expcomp reached target.")
            (Actor|Tick|SetActorTickEnabled false)))))
    (:then_2
      (Utilities|IsValid _postprocessvolume
        (:Is%20Valid
          (Variables|/Script/Engine.PostProcessVolume|SetSettings _postprocessvolume (Utilities|Struct|MakePostProcessSettings (Math|Interpolation|FInterptoConstant (.exposureCompensation (Utilities|Struct|BreakWeatherParams (Variables|Default|GetcurrentWeatherParams))) (.exposureCompensation (Utilities|Struct|BreakWeatherParams (LocalVariables|GettargetWeatherParams))) (Utilities|Time|GetWorldDeltaSeconds) (Variables|Default|GetweatherChangeSpeed))))
          (Development|PrintString (Utilities|String|ToString(Float) (Math|Interpolation|FInterptoConstant (.exposureCompensation (Utilities|Struct|BreakWeatherParams (Variables|Default|GetcurrentWeatherParams))) (.exposureCompensation (Utilities|Struct|BreakWeatherParams (LocalVariables|GettargetWeatherParams))) (Utilities|Time|GetWorldDeltaSeconds) (Variables|Default|GetweatherChangeSpeed)))))))
    (:then_3
      (Utilities|IsValid _skyatmosphere
        (:Is%20Valid
          (Class|SkyAtmosphereComponent|SetRayleighScattering (Variables|/Script/Engine.SkyAtmosphere|GetSkyAtmosphereComponent _skyatmosphere) (CallFunction|ColorFinterptoConstant (.rayleighScattering (Utilities|Struct|BreakWeatherParams (Variables|Default|GetcurrentWeatherParams))) (.rayleighScattering (Utilities|Struct|BreakWeatherParams (LocalVariables|GettargetWeatherParams))) (Variables|Default|GetweatherChangeSpeed))))))))

(fn ColorFinterptoConstant
  (params (currentColor :type Linear%20Color%20Structure) (targetColor :type Linear%20Color%20Structure) (finterpSpeed :type Float%20%28double-precision%29))
  (bind (_r _g _b _a) (Math|Color|BreakColor currentColor))
  (bind (_r_2 _g_2 _b_2 _a_2) (Math|Color|BreakColor targetColor))
  (bind _returnvalue (Utilities|Time|GetWorldDeltaSeconds))
  (return (Utilities|Struct|MakeLinearColor (Math|Interpolation|FInterptoConstant _r _r_2 _returnvalue finterpSpeed) (Math|Interpolation|FInterptoConstant _g _g_2 _returnvalue finterpSpeed) (Math|Interpolation|FInterptoConstant _b _b_2 _returnvalue finterpSpeed) (Math|Interpolation|FInterptoConstant _a _a_2 _returnvalue finterpSpeed))))

(fn ShouldChangeAtmosphere
  (params (currentWeather :type WeatherPresets%20Enum :default "NewEnumerator0") (targetWeather :type WeatherPresets%20Enum :default "NewEnumerator0"))
  (return (not (Utilities|Enum|Equal(Enum) currentWeather targetWeather))))

(fn TempChangeGlobalStruct
  (Utilities|Struct|SetmembersinWeatherParams (Variables|Default|GetcurrentWeatherParams) 1.2e+02))

(fn CheckandChangeAtmosphere
  (params (targetWeatherPreset :type WeatherPresets%20Enum :default "NewEnumerator0"))
  (bind _output_get (Variables|Default|SettargetWeatherPreset targetWeatherPreset))
  (bind _shouldchangeatmosphere (CallFunction|ShouldChangeAtmosphere (Variables|Default|GetcurrentWeatherPreset) _output_get))
  (if _shouldchangeatmosphere
    (Utilities|Struct|SetmembersinWeatherParams (Variables|Default|GetcurrentWeatherParams) (Variables|Default|GettargetWeatherPreset))
    (Variables|Default|SetcurrentWeatherPreset (Variables|Default|GettargetWeatherPreset))
    (Actor|Tick|SetActorTickEnabled true)))